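; HUD for the racing game that draws the lap time and a leaderboard of the three best laps.
; BeginPlay caches the BP_RacingGameMode, and DrawHUD reads its times each frame to draw color-coded text at fixed screen positions, with a rectangle behind the leaderboard.
; A Float->Time graph holds integer math that splits tenths of a second into a colon-separated hours, minutes, seconds and tenths string.
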(event EventBeginPlay
  (bind _asbp_racing_game_mode (Utilities|Casting|CastToBP_RacingGameMode (Game|GetGameMode)))
  (Variables|Default|SetRacingGameMode _asbp_racing_game_mode))

(event EventDrawHUD
  (params (SizeX :type Integer) (SizeY :type Integer))
  (bind _racinggamemode (Variables|Default|GetRacingGameMode))
  (HUD|DrawText (Utilities|Float->Time (Variables|/Game/Blueprints/BP_RacingGameMode.BP_RacingGameMode_C|GetLapTime (Variables|Default|GetRacingGameMode))) "(R=1.000000,G=0.000000,B=0.000000,A=1.000000)" 1e+03 6.5e+02 0 3.0 false)
  (HUD|DrawRect "(R=0,G=0,B=0,A=1)" 9.9e+02 1e+01 1.6e+02 1.5e+02)
  (HUD|DrawText "Best Laps" "(R=1.000000,G=0.000000,B=0.000000,A=1.000000)" 1e+03 1e+01 0 2.0 false)
  ;[1 1 1] Comment
  (HUD|DrawText (Utilities|String|Append "1)" (Utilities|Float->Time (Variables|/Game/Blueprints/BP_RacingGameMode.BP_RacingGameMode_C|GetBestLap1 _racinggamemode))) "(R=1.000000,G=1.000000,B=0.000000,A=1.000000)" 1e+03 4e+01 0 2.0 false)
  (HUD|DrawText (Utilities|String|Append "2)" (Utilities|Float->Time (Variables|/Game/Blueprints/BP_RacingGameMode.BP_RacingGameMode_C|GetBestLap2 _racinggamemode))) "(R=0.600000,G=0.600000,B=0.600000,A=1.000000)" 1e+03 7e+01 0 2.0 false)
  (HUD|DrawText (Utilities|String|Append "3)" (Utilities|Float->Time (Variables|/Game/Blueprints/BP_RacingGameMode.BP_RacingGameMode_C|GetBestLap3 _racinggamemode))) "(R=0.494792,G=0.136422,B=0.000000,A=1.000000)" 1e+03 1e+02 0 2.0 false))

(fn ConstructionScript)