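; BP_RacingGameMode is the game mode for a racing game that times laps and keeps the three best lap times.
; StartGame resets state on BeginPlay and starts a looping Clock timer that counts LapTime in tenths of a second.
; CheckPointReached advances the checkpoint index for equal or higher numbers, printing it.
; Reaching checkpoint 0 after 8 completes a lap, slotting LapTime into the ranking and restarting the count.
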(event Custom|Clock
  (Variables|Default|SetLapTime (+ (Variables|Default|GetLapTime) 1)))

(event Custom|CheckPointReached
  (params (CheckPoint :type Integer))
  (if (>= CheckPoint (Variables|Default|GetCheckpointIndex))
    (Variables|Default|SetLastCheckPoint (Variables|Default|GetCheckpointIndex))
    (bind _output_get (Variables|Default|SetCheckpointIndex CheckPoint))
    (Development|PrintString (Utilities|String|ToString(Integer) _output_get))
    (elif (and (== CheckPoint 0) (== (Variables|Default|GetCheckpointIndex) 8))
      (Variables|Default|SetCheckpointIndex CheckPoint)
      (if (< (Variables|Default|GetLapTime) (Variables|Default|GetBestLap1))
        (Variables|Default|SetBestLap3 (Variables|Default|GetBestLap2))
        (Variables|Default|SetBestLap2 (Variables|Default|GetBestLap1))
        (Variables|Default|SetBestLap1 (Variables|Default|GetLapTime))
        (elif (< (Variables|Default|GetLapTime) (Variables|Default|GetBestLap2))
          (Variables|Default|SetBestLap3 (Variables|Default|GetBestLap2))
          (Variables|Default|SetBestLap2 (Variables|Default|GetLapTime))
          (elif (< (Variables|Default|GetLapTime) (Variables|Default|GetBestLap3))
            (Variables|Default|SetBestLap3 (Variables|Default|GetLapTime)))))
      (Variables|Default|SetLapTime 0))))

(event EventBeginPlay
  (Utilities|StartGame))

(fn ConstructionScript)