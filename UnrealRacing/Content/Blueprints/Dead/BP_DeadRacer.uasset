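; BP_DeadRacer is a drivable car that turns player input into vehicle control and camera orbit.
; Throttle and steering axes feed straight into the VehicleMovement component, and the Emergency Break action holds the handbrake while pressed.
; Mouse X and Y add relative yaw and pitch to the CameraBoom, with no clamping or scaling in the graph.
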(event Input|ActionEvents|InputActionEmergencyBreak
  (params (Key :type Key%20Structure :default "None"))
  (bind _vehiclemovement (Variables|Default|GetVehicleMovement))
  ;[1 1 1] Set Input for Car
  (:Pressed
    (Class|WheeledVehicleMovementComponent|SetHandbrakeInput _vehiclemovement true))
  (:Released
    (Class|WheeledVehicleMovementComponent|SetHandbrakeInput _vehiclemovement false)))

(event Input|AxisEvents|InputAxisMoveForward
  (params (AxisValue :type Float%20%28single-precision%29))
  ;[1 1 1] Set Input for Car
  (Class|WheeledVehicleMovementComponent|SetThrottleInput (Variables|Default|GetVehicleMovement) AxisValue))

(event Input|AxisEvents|InputAxisSteering
  (params (AxisValue :type Float%20%28single-precision%29))
  ;[1 1 1] Set Input for Car
  (Class|WheeledVehicleMovementComponent|SetSteeringInput (Variables|Default|GetVehicleMovement) AxisValue))

(event Input|MouseEvents|MouseX
  (params (AxisValue :type Float%20%28single-precision%29))
  ;[1 1 1] Camera
  (Transformation|AddRelativeRotation (Variables|Default|GetCameraBoom) (Math|Rotator|MakeRotator 0.0 0.0 AxisValue) false false))

(event Input|MouseEvents|MouseY
  (params (AxisValue :type Float%20%28single-precision%29))
  ;[1 1 1] Camera
  (Transformation|AddRelativeRotation (Variables|Default|GetCameraBoom) (Math|Rotator|MakeRotator 0.0 AxisValue 0.0) false false))

(fn ConstructionScript)