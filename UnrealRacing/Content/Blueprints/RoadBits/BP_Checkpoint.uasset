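; BP_Checkpoint is a racing checkpoint that reports when the player's racer reaches it.
; On BeginPlay it caches the BP_RacingGameMode and player 0's BP_RacerPawn.
; When that pawn begins overlapping it, it passes its CheckPointIndex to the game mode's CheckPointReached, ignoring all other actors.
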(event Collision|EventActorBeginOverlap
  (params (OtherActor :type Actor%20Object%20Reference))
  (if (== OtherActor (Variables|Default|GetRacer))
    (Default|CheckPointReached (Variables|Default|GetRacingGame) (Variables|Default|GetCheckPointIndex))))

(event EventBeginPlay
  (bind _asbp_racing_game_mode (Utilities|Casting|CastToBP_RacingGameMode (Game|GetGameMode)))
  (Variables|Default|SetRacingGame _asbp_racing_game_mode)
  (bind _asbp_racer_pawn (Utilities|Casting|CastToBP_RacerPawn (Game|Player|GetPlayerPawn 0)))
  (Variables|Default|SetRacer _asbp_racer_pawn))

(fn ConstructionScript)